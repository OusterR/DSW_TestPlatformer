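; BP_Checkpoint_Platformer is a platformer checkpoint that updates the player's respawn transform.
; When an untoggled checkpoint is overlapped by BP_MyPlayer, it stores a point above itself, with its rotation, as RespawnTransform.
; It then passes its index in the Spawner's CheckPoints array to SetCheckpointsToggled.
; ChangeToggled sets the state and recolors the point light green or blue, which the construction script also applies.
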(event `self.ReceiveActorBeginOverlap`
  (params (OtherActor :type "Actor Object Reference"))
  (bind _spawner (`self.Spawner`))
  (if (not (`self.Toggled`))
    (cast `/Game/MyPlatformer/Blueprints/BP_MyPlayer` OtherActor)
    (`self.ChangeSpawnTransform` (`KismetMathLibrary.MakeTransform` (+ (`self.K2_GetActorLocation`) (0.0 0.0 250.0)) (`self.K2_GetActorRotation`)))
    ;[0 0.3166 1] Send Data to Spawner
    (`/Game/MyPlatformer/Blueprints/Interactive_Stuff/BP_CheckPointSpawner_Platformer.SetCheckpointsToggled` _spawner (`KismetArrayLibrary.Array_Find` (`/Game/MyPlatformer/Blueprints/Interactive_Stuff/BP_CheckPointSpawner_Platformer.CheckPoints` _spawner) self))))

(event `ChangeToggled`
  (params (Toggled :type Boolean :default true))
  (set `self.Toggled` Toggled)
  (`self.ChangeColor`))

(fn `ChangeColor`
  (`LightComponent.SetLightColor` (`self.PointLight`) (`KismetMathLibrary.SelectColor` (struct :`R` 0.013801 :`G` 1.0 :`A` 1.0) (struct :`G` 0.50519 :`B` 1.0 :`A` 1.0) (`self.Toggled`)) true))

(fn `ChangeSpawnTransform`
  (params (Transform :type "Transform Structure"))
  (bind _asbp_my_player (cast `/Game/MyPlatformer/Blueprints/BP_MyPlayer` (`GameplayStatics.GetPlayerCharacter` 0)))
  (set `/Game/MyPlatformer/Blueprints/BP_MyPlayer.RespawnTransform` Transform _asbp_my_player))

(fn `UserConstructionScript`
  (`self.ChangeColor`))