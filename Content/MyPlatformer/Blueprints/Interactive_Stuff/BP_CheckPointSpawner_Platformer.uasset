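; Spawner actor that lays out a chain of platformer checkpoints along a spline.
; On BeginPlay it spawns a BP_Checkpoint_Platformer at each spline point, passes itself as Spawner and stores them in point order.
; SetCheckpointsToggled switches on every checkpoint from the first through the given index, so earlier checkpoints are toggled along with that one.
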(event `self.ReceiveBeginPlay`
  (for _index (range (`SplineComponent.GetNumberOfSplinePoints` (`self.Spline`)))
    (bind _returnvalue (`|SpawnActorFromClass` "/Game/MyPlatformer/Blueprints/Interactive_Stuff/BP_Checkpoint_Platformer.BP_Checkpoint_Platformer_C" (`KismetMathLibrary.MakeTransform` (`SplineComponent.GetLocationAtSplinePoint` (`self.Spline`) _index "World")) "AlwaysSpawn" "OverrideRootScale" null self null))
    (`KismetArrayLibrary.Array_AddUnique` (`self.CheckPoints`) _returnvalue)))

(fn `SetCheckpointsToggled`
  (params (Index :type Integer))
  (for _index (range (+ Index 1))
    (`/Game/MyPlatformer/Blueprints/Interactive_Stuff/BP_Checkpoint_Platformer.ChangeToggled` (`|GetArrayItem` (`self.CheckPoints`) _index) true)))

(fn `UserConstructionScript`)