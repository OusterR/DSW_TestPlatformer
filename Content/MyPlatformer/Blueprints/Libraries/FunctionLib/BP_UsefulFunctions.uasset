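; Blueprint function library for the platformer that shows and hides menu widgets and provides two halve-a-value helpers.
; ShowMenu adds a widget to the viewport, marks it active in BP_MyPlayerController's Widgets map, optionally pauses, shows the cursor and disables character input.
; HideMenu removes the widget and marks it inactive, restoring game-only input, character control and unpausing only when no tracked widget remains active.
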(fn `GetHalfValueOf`
  (params (Value :type "Float (double-precision)"))
  (returns (HalfValue :type "Float (double-precision)"))
  (return (/ Value 2.0)))

(fn `HalfOfValue`
  (params (Int :type "Float (double-precision)"))
  (returns (ReturnValue :type "Float (double-precision)"))
  (return (/ Int 2.0)))

(fn `HideMenu`
  (params (Widget :type "UserWidget Object Reference"))
  (locals (`IsAnyWidgetInViewport?` :type Boolean))
  (bind _returnvalue (`GameplayStatics.GetPlayerController` null))
  (`Widget.RemoveFromParent` Widget)
  ;[0 0.3166 1] Update Widgets Map
  (bind _asbp_my_player_controller (cast `/Game/MyPlatformer/Blueprints/BP_MyPlayerController` (`GameplayStatics.GetPlayerController` null)))
  (bind _widgets (`/Game/MyPlatformer/Blueprints/BP_MyPlayerController.Widgets` _asbp_my_player_controller))
  (`BlueprintMapLibrary.Map_Add` _widgets Widget)
  ;[0 0.3166 1] Check if there is any widget in viewport
  (bind _values (`BlueprintMapLibrary.Map_Values` _widgets))
  (for _array_element _values
    (if _array_element
      (set `local.IsAnyWidgetInViewport?` true)
      (break)))
  ;[0 0.3166 1] If no widget in viewport then change to game mode and hide cursor
  (if (not (`local.IsAnyWidgetInViewport?`))
    (`WidgetBlueprintLibrary.SetInputMode_GameOnly` _returnvalue)
    (set `PlayerController.bShowMouseCursor` false _returnvalue)
    ;[0 0.3166 1] Enable Character Input
    (`Actor.EnableInput` (`GameplayStatics.GetPlayerCharacter` null) (`GameplayStatics.GetPlayerController` null))
    ;[0 0.3166 1] Unpause the game
    (`GameplayStatics.SetGamePaused` null)))

(fn `ShowMenu`
  (params (Widget :type "UserWidget Object Reference") (`Pause?` :type Boolean))
  (locals (Widget_Temp :type "UserWidget Object Reference") (Pause_Temp :type Boolean))
  (bind _returnvalue (`GameplayStatics.GetPlayerController` null))
  ;[0 0.3166 1] Init local variables
  (set `local.Widget_Temp` Widget)
  (set `local.Pause_Temp` `Pause?`)
  ;[0 0.3166 1] Add widget to viewport
  (`UserWidget.AddToViewport` (`local.Widget_Temp`) 0)
  ;[0 0.3166 1] Update Widgets Map
  (bind _asbp_my_player_controller (cast `/Game/MyPlatformer/Blueprints/BP_MyPlayerController` (`GameplayStatics.GetPlayerController` null)))
  (`BlueprintMapLibrary.Map_Add` (`/Game/MyPlatformer/Blueprints/BP_MyPlayerController.Widgets` _asbp_my_player_controller) (`local.Widget_Temp`) true)
  ;[0 0.3166 1] Pause game if variable checked
  (`GameplayStatics.SetGamePaused` null (`local.Pause_Temp`))
  ;[0 0.3166 1] Change game mode
  (set `PlayerController.bShowMouseCursor` true _returnvalue)
  (`WidgetBlueprintLibrary.SetInputMode_GameAndUIEx` _returnvalue null "DoNotLock" false)
  ;[0 0.3166 1] Disable Character Input
  (`Actor.DisableInput` (`GameplayStatics.GetPlayerCharacter` null) (`GameplayStatics.GetPlayerController` null)))