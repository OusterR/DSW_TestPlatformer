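; BP_FinishText is a world text actor that announces the winner when the game finishes.
; On BeginPlay it registers an event on its FinishLine reference's finish-game binding and caches the first player's BP_MyPlayer character.
; ChangeText sets the TextRender to that player's uppercased name joined to "WINS!", so it always names player zero.
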(event `self.ReceiveBeginPlay`
  (bind _finishline (`self.FinishLine`)
    (:`then`
      (add `/Game/MyPlatformer/Blueprints/Interactive_Stuff/BP_FinishLine.FinishGame` _finishline (`|CreateDelegate` :!event `ChangeText`))
      (bind _asbp_my_player (cast `/Game/MyPlatformer/Blueprints/BP_MyPlayer` (`GameplayStatics.GetPlayerCharacter` 0)))
      (set `self.Player` _asbp_my_player))
    (:`else`)))

(event `ChangeText`
  (`TextRenderComponent.K2_SetText` (`self.TextRender`) (`KismetTextLibrary.Conv_StringToText` (`KismetStringLibrary.Concat_StrStr` (`KismetStringLibrary.ToUpper` (`/Game/MyPlatformer/Blueprints/BP_MyPlayer.PlayerName` (`self.Player`))) " WINS!"))))

(fn `UserConstructionScript`)