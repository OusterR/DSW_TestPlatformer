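; Base moving platform that slides its mesh along a spline, forward when its button state is enabled and back when disabled.
; A looping timer advances a clamped alpha by speed and direction, clearing itself at either spline end.
; A DoOnce and FlipFlop handle direction switching for looped platforms.
; The construction script sets mesh X/Y scale, and an older Timeline-based mover is left unconnected.
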(event `/Game/MyPlatformer/Blueprints/Interfaces/BPI_Devices.SetButtonEnabled`
  (params (Enabled :type Boolean))
  (bind _output_get (set `self.ButtonEnabled` Enabled))
  (if _output_get
    (`self.GoUp`)
    (else
      (`self.GoDown`))))

(event `GoUp`
  ;[0.000507 0.501 0] Second (more advanced) version with time change
  (set `self.Direction` 1.0)
  (bind _returnvalue (`KismetSystemLibrary.K2_SetTimerDelegate` (delegate `startmoving`) (`self.RefreshTime`) true :!label _label))
  (set `self.MoveTick` _returnvalue))

(event `GoDown`
  ;[0.000507 0.501 0] Second (more advanced) version with time change
  (set `self.Direction` -1.0)
  (goto _label))

(event `startmoving`
  (bind _movetimer (`self.MoveTimer`))
  ;[0.000507 0.501 0] Second (more advanced) version with time change
  (set `self.MoveTimer` (+ (`self.MoveTimer`) (* (`self.RefreshTime`) (`self.Direction`) (`self.Speed`))))
  (`SceneComponent.K2_SetWorldLocation` (`self.Mesh`) (`SplineComponent.GetLocationAtDistanceAlongSpline` (`self.Spline`) (`KismetMathLibrary.Lerp` 0.0 (`SplineComponent.GetSplineLength` (`self.Spline`)) (`KismetMathLibrary.FClamp` (`self.MoveTimer`))) "World") false false)
  (if (or (>= _movetimer 1.0) (<= _movetimer 0.0))
    (`self.ResetLoop`) ; RSET LOOP
    (`KismetSystemLibrary.K2_ClearAndInvalidateTimerHandle` (`self.MoveTick`))
    (else
      ;;[0 0.3166 1] Loop
      (`/Engine/EditorBlueprintResources/StandardMacros.DoOnce` false :!label _label_2
        (:`Completed`
          (if (and (`self.Looped`) (`self.ButtonEnabled`))
            (`/Engine/EditorBlueprintResources/StandardMacros.FlipFlop`
              (:`A`
                (`self.GoDown`))
              (:`B`
                (`self.GoUp`)))))))))

(event `ResetLoop`
  ;[0.000507 0.501 0] Second (more advanced) version with time change
  ;;[0 0.3166 1] Loop
  (goto _label_2 :!via `Reset`))

(fn `SetScale`
  (params (X_Scale :type "Float (double-precision)") (Y_Scale :type "Float (double-precision)"))
  (set `self.X_Scale` X_Scale)
  (set `self.Y_Scale` Y_Scale))

(fn `UserConstructionScript`
  (`SceneComponent.SetWorldScale3D` (`self.Mesh`) (`KismetMathLibrary.MakeVector` (`self.X_Scale`) (`self.Y_Scale`) 0.25)))