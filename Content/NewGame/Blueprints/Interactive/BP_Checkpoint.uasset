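; BP_Checkpoint is a checkpoint actor that sets the player's saved transform when a BP_NewPlayer overlaps it while it is untoggled.
; The saved transform uses the checkpoint's rotation and a raised location with unit scale.
; It then passes its index in the Manager's Checkpoints array to SetCheckpointsToggled.
; ChangeToggled updates its state and recolors the point light green or blue, which the construction script also applies.
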(event `self.ReceiveActorBeginOverlap`
  (params (OtherActor :type "Actor Object Reference"))
  (bind (_returnvalue_location _returnvalue_rotation) (`KismetMathLibrary.BreakTransform` (`self.GetTransform`)))
  (bind _manager (`self.Manager`))
  (if (not (`self.Toggled`))
    (bind _asbp_new_player (cast `/Game/NewGame/Blueprints/BP_NewPlayer` OtherActor))
    (set `/Game/NewGame/Blueprints/BP_NewPlayer.PlayerTransform` (`KismetMathLibrary.MakeTransform` (+ _returnvalue_location (0.0 0.0 250.0)) _returnvalue_rotation) _asbp_new_player)
    (`/Game/NewGame/Blueprints/Interactive/BP_CheckpointManager.SetCheckpointsToggled` _manager (`KismetArrayLibrary.Array_Find` (`/Game/NewGame/Blueprints/Interactive/BP_CheckpointManager.Checkpoints` _manager) self))))

(event `ChangeToggled`
  (params (Toggled :type Boolean))
  (set `self.Toggled` Toggled)
  (`self.Change Color`))

(fn `Change Color`
  (`LightComponent.SetLightColor` (`self.PointLight`) (`KismetMathLibrary.SelectColor` (struct :`R` 0.597827 :`G` 1.0 :`A` 1.0) (struct :`G` 0.639754 :`B` 1.0 :`A` 1.0) (`self.Toggled`)) true))

(fn `UserConstructionScript`
  (`self.Change Color`))