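; TestCube is a test Blueprint that launches its Cube component with physics impulses when play begins.
; On BeginPlay, a sequence applies two equally strong impulses to Cube, first from Scene1 and then from Scene.
; Each scene component acts as a thruster marker, with its world location setting the point of application and its forward vector setting the direction.
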(event `self.ReceiveBeginPlay`
  (bind _scene1 (`self.Scene1`))
  (bind _scene (`self.Scene`))
  (`|ExecutionSequence`
    (:`then_0`
      (`PrimitiveComponent.AddImpulseAtLocation` (`self.Cube`) (* (`KismetMathLibrary.GetForwardVector` (`SceneComponent.K2_GetComponentRotation` _scene1)) 40000.0) (`SceneComponent.K2_GetComponentLocation` _scene1) "None"))
    (:`then_1`
      (`PrimitiveComponent.AddImpulseAtLocation` (`self.Cube`) (* (`KismetMathLibrary.GetForwardVector` (`SceneComponent.K2_GetComponentRotation` _scene)) 40000.0) (`SceneComponent.K2_GetComponentLocation` _scene) "None"))))

(fn `UserConstructionScript`)