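; Floor-style button that sinks when actors overlap it and tells AffectedActor its on/off state through BPI_ButtonMechanics.
; In HoldMode an overlap counter keeps it pressed until the last actor leaves; otherwise overlaps toggle it through a FlipFlop gated by GetOverlapped.
; A timeline lerps the Top component down or back, sending the state when finished.
; Each overlap also calls a test function on BP_NewPlayer.
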(event `self.ReceiveBeginPlay`
  ;[0 0.3166 1] Init Top Location
  (set `self.StartLocation` (`SceneComponent.RelativeLocation` (`self.Top`))))

(event `self.ReceiveActorBeginOverlap`
  (params (OtherActor :type "Actor Object Reference"))
  (bind _affectedactor (`self.AffectedActor`))
  (bind _startlocation (`self.StartLocation`))
  ;[1 0.6769 0] Test dispatcher
  (bind _asbp_new_player (cast `/Game/NewGame/Blueprints/BP_NewPlayer` (`GameplayStatics.GetPlayerCharacter` 0)))
  (`/Game/NewGame/Blueprints/BP_NewPlayer.Test` _asbp_new_player)
  (if (`self.HoldMode`)
    (`/Engine/EditorBlueprintResources/StandardMacros.IncrementInt` (`self.OverlappedCount`)
      (:`  `
        (set `self.ButtonEnabled` true :!label _label)
        (bind (_direction _alpha) (`Timeline|Button_Timeline` :!label _label_2)
          (:`Update`
            (`SceneComponent.K2_SetRelativeLocation` (`self.Top`) (`KismetMathLibrary.VLerp` _startlocation (+ _startlocation (0.0 0.0 -4.5)) _alpha) false true))
          (:`Finished`
            ;[0 0.3166 1] Turn On/Off button mechanics
            (if (`KismetSystemLibrary.DoesImplementInterface` _affectedactor "/Game/NewGame/Blueprints/Interface/BPI_ButtonMechanics.BPI_ButtonMechanics_C")
              (message `/Game/NewGame/Blueprints/Interface/BPI_ButtonMechanics.SetButtonActivated` _affectedactor (`self.ButtonEnabled`)))))))
    (elif (`self.GetOverlapped` 1)
      (`/Engine/EditorBlueprintResources/StandardMacros.FlipFlop`
        (:`A`
          (goto _label))
        (:`B`
          (set `self.ButtonEnabled` false :!label _label_3)
          (goto _label_2 :!via `Reverse`))))))

(event `self.ReceiveActorEndOverlap`
  (params (OtherActor :type "Actor Object Reference"))
  (if (`self.HoldMode`)
    (bind _result (`/Engine/EditorBlueprintResources/StandardMacros.DecrementInt` (`self.OverlappedCount`))
      (:`  `
        (if (<= _result 0)
          (goto _label_3))))))

(fn `UserConstructionScript`)