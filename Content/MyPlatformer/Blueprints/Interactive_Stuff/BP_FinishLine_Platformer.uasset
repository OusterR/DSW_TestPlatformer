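; Finish line trigger for the platformer that ends the game when BP_MyPlayer overlaps it.
; The first player overlap calls the FinishGame dispatcher, with a DoOnce preventing repeats.
; The actor binds to that dispatcher itself and, after a configurable delay, shows an end screen widget created at BeginPlay, without pausing.
; The construction script sizes the box from the Size variable.
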(event `self.ReceiveBeginPlay`
  (add `self.FinishGame` (delegate `BindFinishGame`)) ; Listen to FinishGame dispatcher
  ;[0 0.3166 1] Init EndScreen Widget
  (bind _returnvalue (`|CreateWidget` "/Game/MyPlatformer/UI/Widget_EndScreen.Widget_EndScreen_C"))
  (set `self.EndScreen` _returnvalue))

(event `BindFinishGame`
  (`self.ShowEndScreen`))

(event `self.ReceiveActorBeginOverlap`
  (params (OtherActor :type "Actor Object Reference"))
  (cast `/Game/MyPlatformer/Blueprints/BP_MyPlayer` OtherActor) ; If overlapped actor is MyPlayer
  (`/Engine/EditorBlueprintResources/StandardMacros.DoOnce` false
    (:`Completed`
      (`self.FinishGame`) ; Call dispatcher FinishGame
    )))

(event `ShowEndScreen`
  ;[0 0.3166 1] Show EndScreen with delay
  (`KismetSystemLibrary.Delay` (`self.ShowMenuDelay`))
  (`/Game/MyPlatformer/Blueprints/Libraries/FunctionLib/BP_UsefulFunctions.ShowMenu` (`self.EndScreen`)))

(fn `UserConstructionScript`
  (`BoxComponent.SetBoxExtent` (`self.Box`) (`self.Size`) true))