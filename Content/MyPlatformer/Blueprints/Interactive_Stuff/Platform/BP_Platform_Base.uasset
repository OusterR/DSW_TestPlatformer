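; Base moving-platform Blueprint whose mesh travels along a spline when enabled and returns when disabled.
; SetButtonEnabled plays or reverses a timeline whose alpha sets the mesh's distance along the spline.
; An alternative timer-driven version steps a clamped MoveTimer by speed and duration, but its timer setup is disconnected.
; The construction script scales the mesh from X/Y variables with fixed thickness; SetScale stores those variables.
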(event `/Game/MyPlatformer/Blueprints/Interfaces/BPI_Devices.SetButtonEnabled`
  (params (Enabled :type Boolean))
  (if Enabled
    (bind (_direction _alpha) (`Timeline|MoveAlongSpline_Timeline` :!label _label)
      (:`Update`
        (`SceneComponent.K2_SetWorldLocation` (`self.Mesh`) (`SplineComponent.GetLocationAtDistanceAlongSpline` (`self.Spline`) (`KismetMathLibrary.Lerp` 0.0 (`SplineComponent.GetSplineLength` (`self.Spline`)) _alpha) "World") false true)))
    (else
      (goto _label :!via `Reverse`))))

(event `startmoving`
  (bind _movetimer (`self.MoveTimer`))
  ;[0.000507 0.501 0] Second (more advanced) version with time change
  (set `self.MoveTimer` (+ (`self.MoveTimer`) (/ (* (`self.RefreshTime`) (`self.SpeedMultiplier`)) (`self.Time`))))
  (`SceneComponent.K2_SetWorldLocation` (`self.Mesh`) (`SplineComponent.GetLocationAtDistanceAlongSpline` (`self.Spline`) (`KismetMathLibrary.Lerp` 0.0 (`SplineComponent.GetSplineLength` (`self.Spline`)) (`KismetMathLibrary.FClamp` (`self.MoveTimer`))) "World") false true)
  (if (or (>= _movetimer 1.0) (<= _movetimer 0.0))
    (`KismetSystemLibrary.K2_ClearAndInvalidateTimerHandle` (`self.MoveTick`))))

(fn `SetScale`
  (params (X_Scale :type "Float (double-precision)") (Y_Scale :type "Float (double-precision)"))
  (set `self.X_Scale` X_Scale)
  (set `self.Y_Scale` Y_Scale))

(fn `UserConstructionScript`
  (`SceneComponent.SetWorldScale3D` (`self.Mesh`) (`KismetMathLibrary.MakeVector` (`self.X_Scale`) (`self.Y_Scale`) 0.25)))