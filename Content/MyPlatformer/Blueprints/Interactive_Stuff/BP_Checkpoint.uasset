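; BP_Checkpoint is a platformer checkpoint that moves the player's respawn point and signals activation with a point light.
; Its first overlap passes a DoOnce before the BP_MyPlayer cast, so any actor uses up the single trigger.
; For the player, it turns the light from blue to green and sets player 0's RespawnTransform above the checkpoint, matching its rotation.
; The construction script applies the light color from the Toggled state.
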(event `self.ReceiveActorBeginOverlap`
  (params (OtherActor :type "Actor Object Reference"))
  (`/Engine/EditorBlueprintResources/StandardMacros.DoOnce` false
    (:`Completed`
      (cast `/Game/MyPlatformer/Blueprints/BP_MyPlayer` OtherActor)
      (set `self.Toggled` true)
      (`self.ChangeColor`)
      (`self.ChangeSpawnLocation` (`KismetMathLibrary.MakeTransform` (+ (`self.K2_GetActorLocation`) (0.0 0.0 250.0)) (`self.K2_GetActorRotation`))))))

(event `ChangeColor`
  ;[0 0.3166 1] Change color
  (`LightComponent.SetLightColor` (`self.PointLight`) (`KismetMathLibrary.SelectColor` (struct :`R` 0.013801 :`G` 1.0 :`A` 1.0) (struct :`G` 0.50519 :`B` 1.0 :`A` 1.0) (`self.Toggled`)) true))

(event `ChangeSpawnLocation`
  (params (RespawnTransform :type "Transform Structure"))
  ;[0 0.3166 1] Change spawn location
  (bind _asbp_my_player (cast `/Game/MyPlatformer/Blueprints/BP_MyPlayer` (`GameplayStatics.GetPlayerCharacter` 0)))
  (set `/Game/MyPlatformer/Blueprints/BP_MyPlayer.RespawnTransform` RespawnTransform _asbp_my_player))

(fn `UserConstructionScript`
  (`self.ChangeColor`))