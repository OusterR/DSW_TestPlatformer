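; Base moving platform that slides a cube along a spline when SetButtonActivated enables it, and back when disabled.
; A looping timer steps a normalized distance by Speed and direction, placing the cube at that fraction of the spline length.
; At either end the timer is cleared, or a FlipFlop switches direction when Loop and Enabled are set.
; The construction script sets the cube's footprint from ScaleX and ScaleY; an older Timeline-based movement remains unconnected.
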(event `/Game/NewGame/Blueprints/Interface/BPI_ButtonMechanics.SetButtonActivated`
  (params (Enabled :type Boolean))
  (bind _output_get (set `self.Enabled` Enabled))
  (if _output_get
    (`self.PlayAnim`)
    (else
      (`self.ReverseAnim`))))

(event `PlayAnim`
  (set `self.Direction` 1.0)
  (bind _returnvalue (`KismetSystemLibrary.K2_SetTimerDelegate` (delegate `StartMovingPlatform`) (`self.RefreshTime`) true :!label _label))
  (set `self.Timer` _returnvalue))

(event `ReverseAnim`
  (set `self.Direction` -1.0)
  (goto _label))

(event `StartMovingPlatform`
  (bind _distance (`self.Distance`))
  (set `self.Distance` (+ (`self.Distance`) (* (`self.RefreshTime`) (`self.Direction`) (`self.Speed`))))
  (`SceneComponent.K2_SetWorldLocation` (`self.Cube`) (`SplineComponent.GetLocationAtDistanceAlongSpline` (`self.Spline`) (`KismetMathLibrary.Lerp` 0.0 (`SplineComponent.GetSplineLength` (`self.Spline`)) (`KismetMathLibrary.FClamp` (`self.Distance`) 0.0 1.0)) "World") false false)
  (if (or (>= _distance 1.0) (<= _distance 0.0))
    (if (and (`self.Loop`) (`self.Enabled`))
      (`/Engine/EditorBlueprintResources/StandardMacros.FlipFlop`
        (:`A`
          (`self.ReverseAnim`))
        (:`B`
          (`self.PlayAnim`)))
      (else
        (`KismetSystemLibrary.K2_ClearAndInvalidateTimerHandle` (`self.Timer`))))))

(fn `UserConstructionScript`
  ;[0 0.3166 1] Platform shape
  (`SceneComponent.SetWorldScale3D` (`self.Cube`) (`KismetMathLibrary.MakeVector` (`self.ScaleX`) (`self.ScaleY`) 0.1)))