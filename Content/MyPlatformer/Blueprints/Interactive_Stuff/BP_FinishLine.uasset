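; BP_FinishLine is a finish-line trigger actor whose box extent is set from a Size variable in the construction script.
; On overlap, a DoOnce gate runs before the BP_MyPlayer cast, so the first overlapping actor of any type consumes it.
; A player passing both calls the FinishGame dispatcher, bound at BeginPlay to a handler that currently only prints "Finish".
; BeginPlay also caches the player character.
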(event `self.ReceiveBeginPlay`
  (add `self.FinishGame` (delegate `BindFinishGame`))
  ;[0 0.3166 1] Set Player
  (bind _asbp_my_player (cast `/Game/MyPlatformer/Blueprints/BP_MyPlayer` (`GameplayStatics.GetPlayerCharacter` 0)))
  (set `self.Player` _asbp_my_player))

(event `BindFinishGame`
  (`self.FinishGameEvent`))

(event `self.ReceiveActorBeginOverlap`
  (params (OtherActor :type "Actor Object Reference"))
  (`/Engine/EditorBlueprintResources/StandardMacros.DoOnce` false
    (:`Completed`
      (cast `/Game/MyPlatformer/Blueprints/BP_MyPlayer` OtherActor)
      (`self.FinishGame`))))

(event `FinishGameEvent`
  (`KismetSystemLibrary.PrintString` "Finish"))

(fn `UserConstructionScript`
  (`BoxComponent.SetBoxExtent` (`self.Box`) (`self.Size`) true))