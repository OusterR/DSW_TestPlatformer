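; BP_Button is an overlap-triggered pressure button that enables or disables an assigned AffectedActor.
; HoldMode keeps it pressed until the overlap count reaches zero; otherwise overlaps alternate on and off through a FlipFlop.
; Toggle mode filters double presses with a short delay and an overlapping-actor count check, which prints debug text.
; A timeline lowers or raises TopMesh, then sends the state via BPI_Devices when finished.
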(event `self.ReceiveBeginPlay`
  ;[0 0.3166 1] Default (Start) Location
  (set `self.StartLoc` (`SceneComponent.RelativeLocation` (`self.TopMesh`))))

(event `self.ReceiveActorBeginOverlap`
  (params (OtherActor :type "Actor Object Reference"))
  (bind _startloc (`self.StartLoc`))
  (bind _affectedactor (`self.AffectedActor`))
  (if (`self.HoldMode`)
    (`/Engine/EditorBlueprintResources/StandardMacros.IncrementInt` (`self.OverlappingCount`)
      (:`  `
        (set `self.EnableButton` true :!label _label)
        ;[0 0.3166 1] Button (turn on / turn off) animation
        (bind (_direction _alpha) (`Timeline|Button_Timeline` :!label _label_2)
          (:`Update`
            (`SceneComponent.K2_SetRelativeLocation` (`self.TopMesh`) (`KismetMathLibrary.VLerp` _startloc (+ _startloc (0.0 0.0 -70.0)) _alpha) false true))
          (:`Finished`
            ;[0 0.3166 1] Turn On/Off button mechanics
            (if (`KismetSystemLibrary.DoesImplementInterface` _affectedactor "/Game/MyPlatformer/Blueprints/Interfaces/BPI_Devices.BPI_Devices_C")
              (message `/Game/MyPlatformer/Blueprints/Interfaces/BPI_Devices.SetButtonEnabled` _affectedactor (`self.EnableButton`)))))))
    (else
      (`KismetSystemLibrary.Delay` 0.2) ; Double press fix
      (if (`self.Is Overlapping` 1)
        (`/Engine/EditorBlueprintResources/StandardMacros.FlipFlop`
          (:`A`
            (goto _label))
          (:`B`
            (set `self.EnableButton` false :!label _label_3)
            (goto _label_2 :!via `Reverse`)))))))

(event `self.ReceiveActorEndOverlap`
  (params (OtherActor :type "Actor Object Reference"))
  (if (`self.HoldMode`)
    (bind _result (`/Engine/EditorBlueprintResources/StandardMacros.DecrementInt` (`self.OverlappingCount`))
      (:`  `
        (if (<= _result 0)
          (goto _label_3))))))

(fn `Is Overlapping`
  (params (MaxLength :type Integer))
  (returns (ReturnValue :type Boolean))
  (bind _returnvalue (<= (`KismetArrayLibrary.Array_Length` (`self.GetOverlappingActors` null)) MaxLength))
  (`KismetSystemLibrary.PrintString` (`KismetStringLibrary.Concat_StrStr` "mniej niz " (`KismetStringLibrary.Conv_IntToString` MaxLength) " result: " (`KismetStringLibrary.Conv_BoolToString` _returnvalue)) true true (struct :`G` 0.66 :`B` 1.0 :`A` 1.0) 6.0)
  (return _returnvalue))

(fn `UserConstructionScript`)